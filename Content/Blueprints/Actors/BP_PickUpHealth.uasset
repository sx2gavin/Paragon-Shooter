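; BP_PickUpHealth is a health pickup actor whose graph only handles a launch motion at BeginPlay, with no collection or healing logic.
; It caches its location, picks a random upper-hemisphere direction and plays the Jump timeline.
; The timeline's vector track drives an offset from the start: X scales travel along the direction's horizontal components, while Z sets height independently.
; Each update sets location without sweeping for collision.
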(event `self.ReceiveBeginPlay`
  (set `self.CachedActorLocation` (`self.K2_GetActorLocation`))
  (set `self.RandomDirection` (`KismetMathLibrary.RandomUnitVectorInConeInDegrees` (0.0 0.0 1.0) 90.0))
  (bind (_direction _jump_location) (`Timeline|Jump`)
    (:`Update`
      (bind (_returnvalue_x _returnvalue_y) (`KismetMathLibrary.BreakVector` (* (`self.RandomDirection`) (* (.x _jump_location) 80.0))))
      (`self.K2_SetActorLocation` (+ (`KismetMathLibrary.MakeVector` _returnvalue_x _returnvalue_y (* (.z _jump_location) 80.0)) (`self.CachedActorLocation`))))))

(fn `UserConstructionScript`)